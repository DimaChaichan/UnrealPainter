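; Test actor in the paint performance tests that bobs vertically on a sine of game time and deals damage to a target actor.
; Its Hit event validates HitActor, line traces to it on Visibility with debug drawing, and applies point damage to whatever the trace strikes.
; AddDamage enters the same trace without the validity check; the timer node that would bind it is never executed.
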(event Custom|Hit
  (params (Time :type Float%20%28single-precision%29))
  (Utilities|IsValid (Variables|Default|GetHitActor)
    (:Is%20Valid
      (bind (_outhit _returnvalue) (Collision|LineTraceByChannel (Transformation|GetActorLocation) (Transformation|GetActorLocation (Variables|Default|GetHitActor)) "TraceTypeQuery1" false 0 "ForDuration" true "(R=1.000000,G=0.000000,B=0.000000,A=1.000000)" "(R=0.000000,G=1.000000,B=0.000000,A=1.000000)" 0.1))
      (if _returnvalue
        (Game|Damage|ApplyPointDamage (.HitActor (Collision|BreakHitResult _outhit)) 1.0 (.TraceStart (Collision|BreakHitResult _outhit)) _outhit)))))

(event Custom|AddDamage
  (bind (_outhit _returnvalue) (Collision|LineTraceByChannel (Transformation|GetActorLocation) (Transformation|GetActorLocation (Variables|Default|GetHitActor)) "TraceTypeQuery1" false 0 "ForDuration" true "(R=1.000000,G=0.000000,B=0.000000,A=1.000000)" "(R=0.000000,G=1.000000,B=0.000000,A=1.000000)" 0.1))
  (if _returnvalue
    (Game|Damage|ApplyPointDamage (.HitActor (Collision|BreakHitResult _outhit)) 1.0 (.TraceStart (Collision|BreakHitResult _outhit)) _outhit)))

(event EventTick
  (params (DeltaSeconds :type Float%20%28single-precision%29))
  (Transformation|SetActorLocation (+ (Math|Vector|MakeVector 0.0 0.0 (* (Math|Trig|Sin(Radians) (Utilities|Time|GetGameTimeinSeconds)) DeltaSeconds 5e+01)) (Transformation|GetActorLocation)) false false))

(fn ConstructionScript)