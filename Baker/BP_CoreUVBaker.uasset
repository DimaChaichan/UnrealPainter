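; BP_CoreUVBaker bakes a static or skeletal mesh's UV data into a render target and saves it as a texture asset in the editor.
; It spawns a temporary mesh component, applies a UV baker material to the chosen slot, and captures only that component with an orthographic SceneCapture2D.
; An optional material pass dilates the capture into a second target.
; Both targets can be saved as HDR static textures.
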(event Custom|AddDilate
  (Utilities|IsValid (Variables|Setup|GetTextureRenderDilate)
    (:Is%20Valid
      (CallFunction|DilateTexture))))

(event Custom|SaveUVTexture
  (bind _texturetargetuvs (Variables|Setup|GetTextureTargetUVs))
  (Utilities|IsValid _texturetargetuvs
    (:Is%20Valid
      (Class|KismetRenderingLibrary|RenderTargetCreateStaticTexture2DEditorOnly _texturetargetuvs "UVsTexture" "TC_HDR" "TMGS_FromTextureGroup"))))

(event Custom|CaptureStaticMesh
  (Utilities|IsValid (Variables|Setup|GetBakeStaticMesh)
    (:Is%20Valid
      (bind _returnvalue (AddComponent|AddStaticMeshComponent false))
      (bind _returnvalue_2 (Components|StaticMesh|SetStaticMesh _returnvalue (Variables|Setup|GetBakeStaticMesh)))
      (if _returnvalue_2
        (CallFunction|Capture _returnvalue)
        (Components|DestroyComponent _returnvalue)
        (else
          (Development|PrintString "Can't set Static Mesh"))))
    (:Is%20Not%20Valid
      (Development|PrintString "Static Mesh ist not set!"))))

(event Custom|CaptureSkeletalMesh
  (Utilities|IsValid (Variables|Setup|GetBakeSkeletalMesh)
    (:Is%20Valid
      (bind _returnvalue (AddComponent|AddSkeletalMeshComponent false))
      (Components|SkeletalMesh|SetSkeletalMeshAsset _returnvalue (Variables|Setup|GetBakeSkeletalMesh))
      (CallFunction|Capture _returnvalue)
      (Components|DestroyComponent _returnvalue))
    (:Is%20Not%20Valid
      (Development|PrintString "Skelatal Mesh ist not set!"))))

(event Custom|SaveDilateTexture
  (bind _texturerenderdilate (Variables|Setup|GetTextureRenderDilate))
  (Utilities|IsValid _texturerenderdilate
    (:Is%20Valid
      (Class|KismetRenderingLibrary|RenderTargetCreateStaticTexture2DEditorOnly _texturerenderdilate "DilateTexture" "TC_HDR" "TMGS_FromTextureGroup"))))

(fn ConstructionScript
  (Variables|/Script/Engine.SceneCaptureComponent2D|SetTextureTarget (Variables|Default|GetSceneCaptureComponent2D) (Variables|Setup|GetTextureTargetUVs))
  (bind _returnvalue (Rendering|Material|CreateDynamicMaterialInstance "/Game/UnrealPainter/Materials/Projector/M_DilateTexture.M_DilateTexture" "None" "None" :!class /Script/Engine.KismetMaterialLibrary))
  (Variables|intern|SetDilateDynMaterial _returnvalue)
  (bind _returnvalue_2 (Rendering|Material|CreateDynamicMaterialInstance "/Game/UnrealPainter/Materials/Projector/M_PaintUVBaker.M_PaintUVBaker" "None" "None" :!class /Script/Engine.KismetMaterialLibrary))
  (Variables|Intern|SetBakerDynMaterial _returnvalue_2))

(fn Capture
  (params (Target :type Primitive%20Component%20Object%20Reference))
  (bind _bakerdynmaterial (Variables|Intern|GetBakerDynMaterial))
  (Utilities|IsValid (Variables|Intern|GetBakerDynMaterial)
    (:Is%20Valid
      (Variables|/Script/Engine.SceneCaptureComponent2D|SetOrthoWidth (Variables|Default|GetSceneCaptureComponent2D) (Math|Conversions|ToFloat(Integer) (Variables|Setup|GetTextureSize)))
      (Rendering|SceneCapture|ClearShowOnlyComponents (Variables|Default|GetSceneCaptureComponent2D))
      (Rendering|SceneCapture|ShowOnlyComponent (Variables|Default|GetSceneCaptureComponent2D) Target)
      (Rendering|Material|SetScalarParameterValue _bakerdynmaterial "TextureSize" (Math|Conversions|ToFloat(Integer) (Variables|Setup|GetTextureSize)) :!class /Script/Engine.MaterialInstanceDynamic)
      (Rendering|Material|SetMaterial Target (Variables|Setup|GetBakeMaterialIndex) _bakerdynmaterial)
      (Rendering|Material|SetVectorParameterValue _bakerdynmaterial "Offset" (Math|Conversions|ToLinearColor(Vector) (Variables|Setup|GetOffset)) :!class /Script/Engine.MaterialInstanceDynamic)
      (Rendering|SceneCapture|CaptureScene (Variables|Default|GetSceneCaptureComponent2D) :!class /Script/Engine.SceneCaptureComponent2D))))

(fn DilateTexture
  (bind _dilatedynmaterial (Variables|intern|GetDilateDynMaterial))
  (Rendering|Material|SetTextureParameterValue _dilatedynmaterial "Mask" (Variables|Setup|GetTextureTargetUVs))
  (Rendering|Material|SetScalarParameterValue _dilatedynmaterial "Steps" (Variables|Setup|GetDiletaSteps) :!class /Script/Engine.MaterialInstanceDynamic)
  (Rendering|Material|SetScalarParameterValue _dilatedynmaterial "TextureSize" (Math|Conversions|ToFloat(Integer) (Variables|Setup|GetTextureSize)) :!class /Script/Engine.MaterialInstanceDynamic)
  (Rendering|DrawMaterialtoRenderTarget (Variables|Setup|GetTextureRenderDilate) _dilatedynmaterial))